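; AT_PC is a player controller that handles the death and respawn of the player's character.
; Its Death event plays a non-looping death animation on the controlled BaseChar's mesh, then unpossesses the pawn.
; After a short delay, it asks AT_GameMode to find a player start and restart the player there.
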(event `Death`
  (bind _returnvalue (`GameplayStatics.GetGameMode`))
  (bind _asbase_char (cast `/Game/BluePrints/Characters/BaseChar` (`self.K2_GetPawn` self)))
  (`SkeletalMeshComponent.PlayAnimation` (`Character.Mesh` _asbase_char) "/Game/Models/Thirdperson/AnimStarterPack/Death_1.Death_1" false)
  (`self.UnPossess`)
  (`KismetSystemLibrary.Delay` 5.0)
  (bind _asat_game_mode (cast `/Game/BluePrints/Game/AT_GameMode` _returnvalue))
  (`GameModeBase.RestartPlayerAtPlayerStart` _returnvalue self (`GameModeBase.K2_FindPlayerStart` _asat_game_mode self ""))
  (`GameModeBase.RestartPlayerAtPlayerStart` _asat_game_mode self (`GameModeBase.K2_FindPlayerStart` _asat_game_mode self "")))

(fn `UserConstructionScript`)